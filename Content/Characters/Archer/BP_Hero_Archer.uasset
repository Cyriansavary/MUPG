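; Archer hero character Blueprint with a dash, a bow attack and a dagger attack.
; Dash passes a CanDash check, routes through server and multicast events for montage and server-side impulse, then clears its flag after a short delay.
; Pressing fire plays the draw montage if arrows remain; releasing decrements ammo without rechecking, then spawns a BP_Arrow launched along camera forward.
; The E key plays the dagger animation only.
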(event `InputAction|Dash`
  (params (Key :type "Key Structure"))
  ;[0 0 0 1 30] Dash
  (:`Pressed`
    (bind _candash (`self.CanDash` :!label _label))
    (if _candash
      (set `self.IsDashing` true)
      (`self.Ability_Dash` (`/Game/Characters/ABP_Hero_Quinn.MoveDirection` (`self.AnimInstance`)))
      (`self.DashCooldown`))))

(event `Dash`
  ;[0 0 0 1 30] Dash
  (goto _label))

(event `self.Ability_Dash`
  (params (Direction :type "/Game/Characters/E_CharMoveDirection Enum" :default "NewEnumerator0"))
  ;[0 0 0 1 30] Dash
  (`/Engine/EditorBlueprintResources/ActorMacros.Switch Has Authority`
    (:`Authority`
      (`self.MC_AbilityDash` "NewEnumerator0"))
    (:`Remote`
      (`self.Svr_AbilityDash` "NewEnumerator0"))))

(event `self.Svr_AbilityDash`
  (params (Direction :type "/Game/Characters/E_CharMoveDirection Enum" :default "NewEnumerator0"))
  ;[0 0 0 1 30] Dash
  (`self.MC_AbilityDash` "NewEnumerator0"))

(event `self.MC_AbilityDash`
  (params (Direction :type "/Game/Characters/E_CharMoveDirection Enum" :default "NewEnumerator0"))
  ;[0 0 0 1 30] Dash
  (`/Game/Characters/ABP_Hero_Quinn.PLayDashMontage` (`self.AnimInstance`) "NewEnumerator0")
  (if (`KismetSystemLibrary.IsServer`)
    (`self.Svr_AddDashImpluse` "NewEnumerator0")))

(event `self.DashCooldown`
  ;[0 0 0 1 30] Dash
  (`KismetSystemLibrary.Delay` 1.0)
  (set `self.IsDashing` false))

(event `Fire`
  ;[0 0 0 1 30] Bow Fire
  (bind _enoughammo (`self.CheckArrowAmmo` :!label _label_2))
  (if _enoughammo
    (`self.Archer_EngageArrowMonatge`)))

(event `InputAction|FireWeapon`
  (params (Key :type "Key Structure"))
  ;[0 0 0 1 30] Bow Fire
  (:`Pressed`
    (goto _label_2))
  (:`Released`
    (set `self.CurrentNbArrow` (- (`self.CurrentNbArrow`) 1))
    (`self.Archer_ArrowFired`)))

(event `Archer_EngageArrowMonatge`
  ;[0 0 0 1 30] Bow Fire
  ;;[1 1 1] Character Animation
  (`|PlayMontage` (`self.Mesh`) (`self.ArrowEngageMontage`)))

(event `Archer_ArrowFired`
  ;[0 0 0 1 30] Bow Fire
  (`|PlayMontage` (`self.Mesh`) (`self.ArrowFiredMontage`)
    (:`then`
      (`self.LaunchArrow`))))

(event `LaunchArrow`
  ;[0 0 0 1 30] Bow Fire
  (bind _returnvalue (`|SpawnActorFromClass` "/Game/Characters/Archer/BowAndArrow/BP_Arrow.BP_Arrow_C" (`SceneComponent.K2_GetComponentToWorld` (`self.WeaponMesh`)) "Undefined" "MultiplyWithRoot" null null))
  (`PrimitiveComponent.AddImpulse` (`/Game/Characters/Archer/BowAndArrow/BP_Arrow.Arrow` _returnvalue) (* (`SceneComponent.GetForwardVector` (`self.Camera`)) (`self.FireForceArrow`)) "None" false))

(event `DaggerAttack`
  ;[0 0 0 1 30] Dagger Attack
  (`self.Archer_DaggerAttackAnimation` :!label _label_3))

(event `Key|E`
  (params (Key :type "Key Structure"))
  ;[0 0 0 1 30] Dagger Attack
  (:`Pressed`
    (goto _label_3)))

(event `Archer_DaggerAttackAnimation`
  ;[0 0 0 1 30] Dagger Attack
  (`SkeletalMeshComponent.PlayAnimation` (`self.Mesh`) (`self.DaggerAttackAnimation`) false))

(fn `CheckArrowAmmo`
  (returns (EnoughAmmo :type Boolean))
  (return (> (`self.CurrentNbArrow`) 0)))

(fn `UserConstructionScript`
  (`parent.UserConstructionScript`))