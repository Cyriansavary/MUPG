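; Shooter game mode that runs a solo or multiplayer endless-wave match against wolf AI.
; It reads travel URL options, waits for expected players to be ready, then spawns each profile's hero at indexed player starts.
; Waves spawn wolves at random tagged points with growing count and health, polling until all die.
; It also handles hero respawns and, when all players are dead, shows game over and server-travels to menu or lobby.
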(event `self.K2_OnLogout`
  (params (ExitingController :type "Controller Object Reference"))
  (bind _asbp_shooter_player_controller (cast `/Game/Framework/BP_Shooter_PlayerController` ExitingController))
  (`KismetArrayLibrary.Array_RemoveItem` (`self.ALL_ConnectedController`) _asbp_shooter_player_controller)
  (`/Engine/EditorBlueprintResources/StandardMacros.DecrementInt` (`self.NumExpectedPlayers`)
    (:`  `
      (`self.UpdateGameStateNames`))))

(event `RespawnAfterDying`
  (params (PlayerController :type "/Game/Framework/BP_Shooter_PlayerController Object Reference"))
  (`Controller.UnPossess` PlayerController)
  (bind _newparam (`self.RespawnPawnForController` PlayerController (`self.K2_FindPlayerStart` PlayerController (`KismetStringLibrary.Conv_IntToString` (`KismetArrayLibrary.Array_Find` (`self.ALL_ConnectedController`) PlayerController)))))
  (`Controller.Possess` PlayerController _newparam))

(event `self.ReceiveBeginPlay`
  (`self.SetGameOption` (`self.OptionsString`))
  (bind _asbp_game_state (cast `/Game/Framework/BP_GameState` (`GameplayStatics.GetGameState`)))
  (set `self.BP Game State` _asbp_game_state)
  (set `self.IsGameModeReady` true))

(event `self.HandleStartingNewPlayer`
  (params (NewPlayer :type "PlayerController Object Reference"))
  (bind _asbp_shooter_player_controller (cast `/Game/Framework/BP_Shooter_PlayerController` NewPlayer))
  (`/Game/Framework/BP_Shooter_PlayerController.LoadProfile` _asbp_shooter_player_controller)
  (`/Game/Framework/BP_Shooter_PlayerController.OnControllerSpawned` _asbp_shooter_player_controller)
  (`KismetArrayLibrary.Array_Add` (`self.ALL_ConnectedController`) _asbp_shooter_player_controller)
  (if (`self.IsGameModeReady`) :!label _label
    (if (`self.IsSoloGame`)
      (bind _allplayersready (`self.CountPlayersSpawned` :!label _label_2))
      (if _allplayersready
        (`self.RestartPlayerAtPlayerStart` (`|GetArrayItem` (`self.ALL_ConnectedController`)) (`self.K2_FindPlayerStart` null "0"))
        (`self.LevelStart_EndlessWave`)
        (else
          (`KismetSystemLibrary.DelayUntilNextTick`)
          (goto _label_2)))
      (elif (== (`self.NumExpectedPlayers`) (`KismetArrayLibrary.Array_Length` (`self.ALL_ConnectedController`)))
        (bind _allplayersready_2 (`self.CountPlayersSpawned` :!label _label_3))
        (if _allplayersready_2
          (for (_array_element _array_index) (`self.ALL_ConnectedController`)
            (`self.RestartPlayerAtPlayerStart` _array_element (`self.K2_FindPlayerStart` _array_element (`KismetStringLibrary.Conv_IntToString` _array_index))))
          (switch `/Game/Framework/E_GameMode` (`self.GameMode`)
            (:`NewEnumerator0`
              (`self.LevelStart_EndlessWave`)))
          (else
            (`KismetSystemLibrary.DelayUntilNextTick`)
            (goto _label_3)))))
    (else
      (`KismetSystemLibrary.DelayUntilNextTick`)
      (goto _label))))

(event `LevelStart_EndlessWave`
  (`self.UpdateGameStateNames`)
  (for _array_element (`self.ALL_ConnectedController`)
    (`/Game/Framework/BP_Shooter_PlayerController.GameStartCount` _array_element))
  (`KismetSystemLibrary.Delay` 1.0)
  (for _array_element_2 (`self.ALL_ConnectedController`)
    (`/Game/Framework/BP_Shooter_PlayerController.EnableAllInput` _array_element_2))
  (bind _outactors (`GameplayStatics.GetAllActorsOfClassWithTag` "/Game/Gameplay/BP_SpawnPoint_AI.BP_SpawnPoint_AI_C" "EndlessWave"))
  (set `self.AllSpawnPoints` _outactors)
  (set `self.GM_EW_NumberWave` 0)
  (set `self.GM_EW_EnemiesHealthThisWave` 100.0)
  (`self.StartWave`))

(event `StartWave`
  (`/Engine/EditorBlueprintResources/StandardMacros.IncrementInt` (`self.GM_EW_NumberWave`)
    (:`  `
      (for _array_element (`self.ALL_ConnectedController`)
        (`/Game/Framework/BP_Shooter_PlayerController.Client_HUD_StartNewWave` _array_element (`self.GM_EW_NumberWave`)))
      (bind _spawncount (`self.GM_EW_GetEnemyCount` (`self.GM_EW_NumberWave`) (`KismetArrayLibrary.Array_Length` (`self.ALL_ConnectedController`))))
      (set `self.GM_EW_NumberOfEnemiesThisWave` _spawncount)
      (bind _enemyhealth (`self.GM_EW_GetEnemyHealth` (`self.GM_EW_NumberWave`)))
      (set `self.GM_EW_EnemiesHealthThisWave` _enemyhealth)
      (`self.WaveSpawning`))))

(event `WaveSpawning`
  (set `self.GM_EW_SpawnCount` 0)
  (bind _returnvalue (`|SpawnActorFromClass` "/Game/AI/BP_AI_Wolf_Base.BP_AI_Wolf_Base_C" (`self.GetTransform` (`KismetArrayLibrary.Array_Random` (`self.AllSpawnPoints`))) "Undefined" "MultiplyWithRoot" null null :!label _label_4))
  (`/Engine/EditorBlueprintResources/StandardMacros.IsValid` _returnvalue
    (:`Is Valid`
      (`/Engine/EditorBlueprintResources/StandardMacros.IncrementInt` (`self.GM_EW_SpawnCount`)
        (:`  `
          (`self.GM_EW_SetupEnemy` _returnvalue)
          (if (== (`self.GM_EW_SpawnCount`) (`self.GM_EW_NumberOfEnemiesThisWave`))
            (set `self.GM_EW_WaitForeEndWave` false :!label _label_5)
            (bind _outactors (`GameplayStatics.GetAllActorsOfClass` "/Game/AI/BP_AI_Wolf_Base.BP_AI_Wolf_Base_C"))
            (for _array_element _outactors
              (if (`/Game/AI/BP_AI_Wolf_Base.IsAlive` _array_element)
                (set `self.GM_EW_WaitForeEndWave` true)
                (break)))
            (if (`self.GM_EW_WaitForeEndWave`)
              (`KismetSystemLibrary.Delay` 0.5)
              (goto _label_5)
              (else
                (`self.WaveIntermission`)))
            (else
              (`KismetSystemLibrary.Delay` (`KismetMathLibrary.Conv_IntToDouble` (/ (`KismetMathLibrary.RandomIntegerInRange` 15 25) 10)))
              (goto _label_4))))))
    (:`Is Not Valid`
      (`KismetSystemLibrary.Delay` 0.2)
      (goto _label_4))))

(event `WaveIntermission`
  (`KismetSystemLibrary.Delay` 3.0)
  (`self.StartWave`))

(event `GM_EW_GameOver`
  (for _array_element (`self.ALL_ConnectedController`)
    (`/Game/Framework/BP_Shooter_PlayerController.ShowGameOverScreen` _array_element (- (`self.GM_EW_NumberWave`) 1)))
  (`KismetSystemLibrary.Delay` 3.0)
  (if (`self.IsSoloGame`)
    (`KismetSystemLibrary.ExecuteConsoleCommand` "servertravel MainMenu_Map" (`GameplayStatics.GetPlayerController` 0))
    (else
      (`KismetSystemLibrary.ExecuteConsoleCommand` "servertravel Lobby_Map" (`GameplayStatics.GetPlayerController` 0)))))

(fn `CountPlayersSpawned`
  (returns (AllPlayersReady :type Boolean))
  (locals (Lcl_PlayerReady :type Integer))
  (for _array_element (`self.ALL_ConnectedController`)
    (if (`/Game/Framework/BP_Shooter_PlayerController.IsPlayerReady` _array_element)
      (`/Engine/EditorBlueprintResources/StandardMacros.IncrementInt` (`local.Lcl_PlayerReady`))))
  (return (== (`local.Lcl_PlayerReady`) (`KismetArrayLibrary.Array_Length` (`self.ALL_ConnectedController`)))))

(fn `GM_EW_GetEnemyCount`
  (params (WaveNumber :type Integer) (NumPlayer :type Integer))
  (returns (SpawnCount :type Integer))
  (locals (Lcl_NewSpawnCount :type Integer))
  (bind _output_get (set `local.Lcl_NewSpawnCount` (+ (+ WaveNumber (* NumPlayer 2)) (`self.GM_EW_NumberOfEnemiesThisWave`))))
  (if (<= _output_get 5)
    (set `local.Lcl_NewSpawnCount` 6))
  (return (`local.Lcl_NewSpawnCount`)))

(fn `GM_EW_GetEnemyHealth`
  (params (WaveNumber :type Integer))
  (returns (EnemyHealth :type "Float (double-precision)"))
  (locals (Lcl_NewHealth :type "Float (double-precision)"))
  (if (== WaveNumber 1)
    (set `local.Lcl_NewHealth` 100.0)
    (else
      (set `local.Lcl_NewHealth` (+ (`self.GM_EW_EnemiesHealthThisWave`) 10.0))))
  (return (`local.Lcl_NewHealth`)))

(fn `GM_EW_Playerdied`
  (locals (Lcl_DeadPlayerCount :type Integer))
  (for _array_element (`self.ALL_ConnectedController`)
    (bind _asbp_hero_base (cast `/Game/Characters/BP_Hero_Base` (`Controller.K2_GetPawn` _array_element)))
    (if (not (`/Game/Characters/BP_Hero_Base.IsAlive` _asbp_hero_base))
      (`/Engine/EditorBlueprintResources/StandardMacros.IncrementInt` (`local.Lcl_DeadPlayerCount`))))
  (if (== (`KismetArrayLibrary.Array_Length` (`self.ALL_ConnectedController`)) (`local.Lcl_DeadPlayerCount`))
    (`self.GM_EW_GameOver`))
  (return))

(fn `GM_EW_SetupEnemy`
  (params (Enemy :type "/Game/AI/BP_AI_Wolf_Base Object Reference"))
  (set `/Game/AI/BP_AI_Wolf_Base.Health` (`self.GM_EW_EnemiesHealthThisWave`) Enemy)
  (return))

(fn `RespawnPawnForController`
  (params (PlayerController :type "/Game/Framework/BP_Shooter_PlayerController Object Reference") (PlayerStart :type "Actor Object Reference"))
  (returns (NewParam :type "Pawn Object Reference"))
  (locals (Lcl_CharClass :type "Actor Class Reference") (Lcl_ModelName :type Name) (Lcl_SkinName :type Name))
  (bind (_s_player_profile_playername _s_player_profile_charrowname _s_player_profile_characterclass _s_player_profile_modelname _s_player_profile_skinname) (break `/Game/SavedData/S_PlayerProfil` (`/Game/Framework/BP_Shooter_PlayerController.S Player Profile` PlayerController)))
  (set `local.Lcl_CharClass` _s_player_profile_characterclass)
  (set `local.Lcl_ModelName` _s_player_profile_modelname)
  (set `local.Lcl_SkinName` _s_player_profile_skinname)
  (bind _returnvalue (`|SpawnActorFromClass` (`local.Lcl_CharClass`) (`self.GetTransform` PlayerStart) "Undefined" "MultiplyWithRoot" null null))
  (bind _asbp_hero_base (cast `/Game/Characters/BP_Hero_Base` _returnvalue))
  (set `/Game/Characters/BP_Hero_Base.ModelName` (`local.Lcl_ModelName`) _asbp_hero_base)
  (set `/Game/Characters/BP_Hero_Base.SkinName` (`local.Lcl_SkinName`) _asbp_hero_base)
  (set `/Game/Characters/BP_Hero_Base.DeathRespawn` true _asbp_hero_base)
  (return _asbp_hero_base))

(fn `SetGameOption`
  (params (GameOptionString :type String))
  (switch `string` (`GameplayStatics.ParseOption` (`local.GameOptionString`) "GameMode")
    (:`EndlessWave`
      (set `self.GameMode` "NewEnumerator0")
      (set `self.NumExpectedPlayers` (`KismetStringLibrary.Conv_StringToInt` (`GameplayStatics.ParseOption` (`local.GameOptionString`) "NumConnectedPlayers")))
      (switch `string` (`GameplayStatics.ParseOption` (`local.GameOptionString`) "IsSoloGame")
        (:`True`
          (set `self.IsSoloGame` true))
        (:`False`
          (set `self.IsSoloGame` false)))
      (switch `string` (`GameplayStatics.ParseOption` (`local.GameOptionString`) "UseSeamlessTravel")
        (:`True`
          (set `self.Seamless Travel Enabled` true)
          (set `self.bUseSeamlessTravel` true))
        (:`False`
          (set `self.Seamless Travel Enabled` false)
          (set `self.bUseSeamlessTravel` false)))
      (return))))

(fn `SpawnDefaultPawnFor`
  (params (NewPlayer :type "Controller Object Reference") (StartSpot :type "Actor Object Reference"))
  (returns (ReturnValue :type "Pawn Object Reference"))
  (locals (Lcl_CharClass :type "Actor Class Reference") (Lcl_ModelName :type Name) (Lcl_SkinName :type Name))
  (bind _asbp_shooter_player_controller (cast `/Game/Framework/BP_Shooter_PlayerController` NewPlayer))
  (bind (_s_player_profile_playername _s_player_profile_charrowname _s_player_profile_characterclass _s_player_profile_modelname _s_player_profile_skinname) (break `/Game/SavedData/S_PlayerProfil` (`/Game/Framework/BP_Shooter_PlayerController.S Player Profile` _asbp_shooter_player_controller)))
  (set `local.Lcl_CharClass` _s_player_profile_characterclass)
  (set `local.Lcl_ModelName` _s_player_profile_modelname)
  (set `local.Lcl_SkinName` _s_player_profile_skinname)
  (bind _returnvalue (`|SpawnActorFromClass` (`local.Lcl_CharClass`) (`self.GetTransform` StartSpot) "Undefined" "MultiplyWithRoot" null null))
  (bind _asbp_hero_base (cast `/Game/Characters/BP_Hero_Base` _returnvalue))
  (set `/Game/Characters/BP_Hero_Base.ModelName` (`local.Lcl_ModelName`) _asbp_hero_base)
  (set `/Game/Characters/BP_Hero_Base.SkinName` (`local.Lcl_SkinName`) _asbp_hero_base)
  (return _asbp_hero_base))

(fn `UpdateGameStateNames`
  (locals (Lcl_AllPlayerNames :type "Array of Text"))
  (for (_array_element _array_index) (`self.ALL_ConnectedController`)
    (`KismetArrayLibrary.Array_Set` (`local.Lcl_AllPlayerNames`) _array_index (`.PlayerName_2_7F780D5844B33835E20C87A4CD3CBC8B` (break `/Game/SavedData/S_PlayerProfil` (`/Game/Framework/BP_Shooter_PlayerController.S Player Profile` _array_element))) true))
  (`/Game/Framework/BP_GameState.Update_HUD_PlayerNames` (`self.BP Game State`) (`local.Lcl_AllPlayerNames`)))

(fn `UserConstructionScript`)